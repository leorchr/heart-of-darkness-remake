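; Snake enemy that watches, attacks and eats the player, or eats a firefly through FFInteract.
; A Tick state machine runs Idle, Looking, Hostile, Attacking and Eating, driven by three nested-purpose overlap volumes for focus, attack and death range.
; It turns its mesh toward the player, swaps material per state and plays audio cues on key transitions.
; Eating the player disables input, then applies damage; attacks and meals end in a cooldown.
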(event `self.ReceiveTick`
  (params (DeltaSeconds :type "Float (single-precision)"))
  (bind _returnvalue (`GameplayStatics.GetPlayerController` 0))
  (bind _audio (`self.Audio`))
  (bind _audio_2 (`self.Audio`))
  (bind _audio_3 (`self.Audio`))
  (bind _audio_4 (`self.Audio`))
  (`parent.ReceiveTick` DeltaSeconds)
  (`|ExecutionSequence`
    (:`then_0`
      (`self.CheckAttackCooldown`))
    (:`then_1`
      ;[0.295 0.7771 1 0.443] Enemy Behavior
      (switch `/Game/DataType/EEnemyState` (`self.EnemyState`)
        (:`NewEnumerator0`
          (if (`self.IsPlayerDetected`)
            (set `self.EnemyState` "NewEnumerator1")
            (`AudioComponent.SetSound` _audio_3 "/Game/Sounds/SFX/Snake/A_Snake_Detect_CUE.A_Snake_Detect_CUE")
            (`AudioComponent.Play` _audio_3 0.0)))
        (:`NewEnumerator1`
          (`self.RotateTowardsPlayer`)
          (if (`self.IsPlayerDetected`)
            (if (`self.IsPlayerInAttackRange`)
              (set `self.EnemyState` "NewEnumerator2"))
            (else
              (set `self.EnemyState` "NewEnumerator0"))))
        (:`NewEnumerator2`
          (if (`self.IsPlayerInAttackRange`)
            (`self.RotateTowardsPlayer`)
            (if (and (not (`self.IsInCoolDown`)) (`self.IsPlayerInDeathRange`))
              (set `self.EnemyState` "NewEnumerator3")
              (`AudioComponent.SetSound` _audio "/Game/Sounds/SFX/Snake/A_Snake_Attack_CUE.A_Snake_Attack_CUE")
              (`AudioComponent.Play` _audio 0.0))
            (else
              (set `self.EnemyState` "NewEnumerator1")
              (`AudioComponent.SetSound` _audio_4 "/Game/Sounds/SFX/Snake/A_Snake_Detect_CUE.A_Snake_Detect_CUE")
              (`AudioComponent.Play` _audio_4 0.0))))
        (:`NewEnumerator3`
          (set `self.AttackTimer` (+ (`self.AttackTimer`) (`GameplayStatics.GetWorldDeltaSeconds`)))
          (if (> (`self.AttackTimer`) (`self.AttackAnimDuration`))
            (if (`self.IsPlayerInDeathRange`)
              (if (> (`/Game/Player/BP_Character_Game.Health` (cast `/Game/Player/BP_Character_Game` (`GameplayStatics.GetPlayerCharacter` 0) :!pure true)) 0.0)
                (set `self.IsPlayerDead` true)
                (set `self.EnemyState` "NewEnumerator5")
                (`AudioComponent.SetSound` _audio_2 null)
                (`AudioComponent.Play` _audio_2 0.0)
                (else
                  (set `self.IsInCoolDown` true :!label _label)
                  (set `self.AttackTimer` 0.0)
                  (set `self.EnemyState` "NewEnumerator2")))
              (else
                (goto _label)))))
        (:`NewEnumerator5`
          (set `self.EatingAnim` true)
          (if (and (`self.IsPlayerDead`) (not (`self.isEatingFirefly`)))
            (`self.DisableInput` _returnvalue _returnvalue))
          (set `self.EatTimer` (+ (`self.EatTimer`) (`GameplayStatics.GetWorldDeltaSeconds`)))
          (if (> (`self.EatTimer`) (`self.EatDuration`))
            (set `self.IsInCoolDown` true)
            (set `self.AttackTimer` 0.0)
            (set `self.EatTimer` 0.0)
            (set `self.EnemyState` "NewEnumerator2")
            (set `self.EatingAnim` false)
            (if (`self.IsPlayerDead`)
              (set `self.IsPlayerDead` false)
              (`GameplayStatics.ApplyDamage` (`GameplayStatics.GetPlayerCharacter` 0) 10.0)
              (else
                (set `self.isEatingFirefly` false)))))))
    (:`then_2`
      (`self.SetupMaterial`))))

(event `self.FocusDetection.OnComponentBeginOverlap`
  (params (OverlappedComponent :type "PrimitiveComponent Object Reference") (OtherActor :type "Actor Object Reference") (OtherComp :type "PrimitiveComponent Object Reference") (OtherBodyIndex :type Integer) (bFromSweep :type Boolean) (SweepResult :type "HitResult Structure (by ref)"))
  ;[1 0.3997 0.9134] Player Detection
  (set `self.IsPlayerDetected` true))

(event `self.AttackDetection.OnComponentBeginOverlap`
  (params (OverlappedComponent :type "PrimitiveComponent Object Reference") (OtherActor :type "Actor Object Reference") (OtherComp :type "PrimitiveComponent Object Reference") (OtherBodyIndex :type Integer) (bFromSweep :type Boolean) (SweepResult :type "HitResult Structure (by ref)"))
  ;[1 0.3997 0.9134] Player Detection
  (set `self.IsPlayerInAttackRange` (`|EnumEquality` (`PrimitiveComponent.GetCollisionObjectType` OtherComp) "ECC_Pawn")))

(event `self.FocusDetection.OnComponentEndOverlap`
  (params (OverlappedComponent :type "PrimitiveComponent Object Reference") (OtherActor :type "Actor Object Reference") (OtherComp :type "PrimitiveComponent Object Reference") (OtherBodyIndex :type Integer))
  ;[1 0.3997 0.9134] Player Detection
  (set `self.IsPlayerDetected` false))

(event `self.AttackDetection.OnComponentEndOverlap`
  (params (OverlappedComponent :type "PrimitiveComponent Object Reference") (OtherActor :type "Actor Object Reference") (OtherComp :type "PrimitiveComponent Object Reference") (OtherBodyIndex :type Integer))
  ;[1 0.3997 0.9134] Player Detection
  (if (`|EnumEquality` (`PrimitiveComponent.GetCollisionObjectType` OtherComp) "ECC_Pawn")
    (set `self.IsPlayerInAttackRange` false)))

(event `self.DeathDetection.OnComponentBeginOverlap`
  (params (OverlappedComponent :type "PrimitiveComponent Object Reference") (OtherActor :type "Actor Object Reference") (OtherComp :type "PrimitiveComponent Object Reference") (OtherBodyIndex :type Integer) (bFromSweep :type Boolean) (SweepResult :type "HitResult Structure (by ref)"))
  ;[1 0.3997 0.9134] Player Detection
  (set `self.IsPlayerInDeathRange` true))

(event `self.DeathDetection.OnComponentEndOverlap`
  (params (OverlappedComponent :type "PrimitiveComponent Object Reference") (OtherActor :type "Actor Object Reference") (OtherComp :type "PrimitiveComponent Object Reference") (OtherBodyIndex :type Integer))
  ;[1 0.3997 0.9134] Player Detection
  (set `self.IsPlayerInDeathRange` false))

(event `self.ReceiveBeginPlay`
  ;[0.3279 1 0.2965] Base Blueprint
  (`parent.ReceiveBeginPlay`)
  (set `self.EnemyState` "NewEnumerator0")
  (set `self.IsPlayerDead` false))

(fn `CheckAttackCooldown`
  (if (`self.IsInCoolDown`)
    (set `self.CooldownTimer` (+ (`self.CooldownTimer`) (`GameplayStatics.GetWorldDeltaSeconds`)))
    (if (> (`self.CooldownTimer`) (`self.CooldownDuration`))
      (set `self.IsInCoolDown` false)
      (set `self.CooldownTimer` 0.0))))

(fn `FFInteract`
  (set `self.EnemyState` "NewEnumerator5")
  (`parent.FFInteract`)
  (set `self.isEatingFirefly` true))

(fn `RotateTowardsPlayer`
  (bind _returnvalue_location (`KismetMathLibrary.BreakTransform` (`self.GetTransform` (`GameplayStatics.GetPlayerPawn` 0))))
  (bind (_returnvalue_roll _returnvalue_pitch _returnvalue_yaw) (`KismetMathLibrary.BreakRotator` (`KismetMathLibrary.FindLookAtRotation` (`SceneComponent.K2_GetComponentLocation` (`self.SM_Ennemys`)) _returnvalue_location)))
  (`SceneComponent.K2_SetWorldRotation` (`self.SM_Ennemys`) (`KismetMathLibrary.RInterpTo` (`SceneComponent.K2_GetComponentRotation` (`self.SM_Ennemys`)) (`KismetMathLibrary.MakeRotator` 0.0 0.0 (+ _returnvalue_yaw 270.0)) (`GameplayStatics.GetWorldDeltaSeconds`) (`self.RotationInterpSpeed`)) false false))

(fn `SetupMaterial`
  (`PrimitiveComponent.SetMaterial` (`self.SM_Ennemys`) 0 (select `/Game/DataType/EEnemyState` (`self.EnemyState`) :`NewEnumerator0` "/Game/Devlopment/Materials/M_EnemyIdle.M_EnemyIdle" :`NewEnumerator1` "/Game/Devlopment/Materials/M_EnemyLooking.M_EnemyLooking" :`NewEnumerator2` "/Game/Devlopment/Materials/M_EnemyHostile.M_EnemyHostile" :`NewEnumerator3` "/Game/Devlopment/Materials/M_EnemyAttacking.M_EnemyAttacking" :`NewEnumerator5` "/Game/Devlopment/Materials/M_EnemyEating.M_EnemyEating" :!type "MaterialInterface Object Reference")))

(fn `UserConstructionScript`
  (`parent.UserConstructionScript`))