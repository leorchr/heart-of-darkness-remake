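; A single firefly actor that wanders around its spawn point and calls FFInteract on any BP_FFInteractable it overlaps.
; Each tick it eases toward a target with VInterpTo, picking a new target once within the acceptance distance.
; Targets come from random horizontal offsets around the spawn position, with a visibility line trace placing them at hover height above the hit surface.
; A missed trace returns the current location, so another pick follows.
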(event `self.ReceiveBeginPlay`
  (set `self.SpawnPosition` (`self.K2_GetActorLocation`))
  (bind _new_position (`self.Find Random Position`))
  (set `self.TargetPosition` _new_position))

(event `self.ReceiveActorBeginOverlap`
  (params (OtherActor :type "Actor Object Reference"))
  (bind _asbp_ffinteractable (cast `/Game/Blueprint/BP_FFInteractable` OtherActor))
  (`/Game/Blueprint/BP_FFInteractable.FFInteract` _asbp_ffinteractable))

(event `self.ReceiveTick`
  (params (DeltaSeconds :type "Float (single-precision)"))
  (if (<= (`KismetMathLibrary.Vector_Distance` (`self.K2_GetActorLocation`) (`self.TargetPosition`)) (`self.DistanceAcceptance`))
    (bind _new_position (`self.Find Random Position`))
    (set `self.TargetPosition` _new_position)
    (else
      (`self.K2_SetActorLocation` (`KismetMathLibrary.VInterpTo` (`self.K2_GetActorLocation`) (`self.TargetPosition`) DeltaSeconds (`self.MaxSpeed`))))))

(fn `Find Random Position`
  (returns (`New Position` :type "Vector Structure"))
  (locals (Return :type "Vector Structure" :default (0.0 0.0 0.0)))
  (bind (_returnvalue_x _returnvalue_y) (`KismetMathLibrary.BreakVector` (`KismetMathLibrary.RandomUnitVector`)))
  (bind _returnvalue (/ (`self.MaxHeight`) 2.0))
  (bind _returnvalue_2 (+ (`self.SpawnPosition`) (* (`KismetMathLibrary.Normal` (`KismetMathLibrary.MakeVector` _returnvalue_x _returnvalue_y)) (`KismetMathLibrary.RandomFloatInRange` 0.0 (`self.MaxDistance`)))))
  ;[1 1 1] Find the correct Height
  (bind (_outhit _returnvalue_3) (`KismetSystemLibrary.LineTraceSingle` :`Start` (+ _returnvalue_2 (`KismetMathLibrary.MakeVector` 0.0 0.0 _returnvalue)) :`End` (- _returnvalue_2 (`KismetMathLibrary.MakeVector` 0.0 0.0 _returnvalue)) :`TraceChannel` "TraceTypeQuery1" :`DrawTime` 1.0))
  (if _returnvalue_3
    (bind (_x _y _z) (`KismetMathLibrary.BreakVector3f` (`.ImpactPoint` (`GameplayStatics.BreakHitResult` _outhit))))
    (set `local.Return` (`KismetMathLibrary.MakeVector` _x _y (+ _z (`self.HoverHeight`))))
    (else
      (set `local.Return` (`self.K2_GetActorLocation`))))
  (return (`local.Return`)))

(fn `UserConstructionScript`)