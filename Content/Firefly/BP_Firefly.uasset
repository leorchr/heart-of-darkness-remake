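; BP_Firefly is an AI-moved firefly character that wanders the level.
; On BeginPlay it applies MaxSpeed to its movement and starts RandomRoam, which moves to a random reachable point within MaxDistance and repeats on each success.
; A FollowPlayer event can move it toward the player while IsSeeingPlayer is set, but its trigger logic is disconnected and the PawnSensing sight event is empty.
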(event `self.PawnSensing.OnSeePawn`
  (params (Pawn :type "Pawn Object Reference")))

(event `Follow Player`
  (if (`self.IsSeeingPlayer?`)
    (`|AIMoveTo` self (0.0 0.0 0.0) (`GameplayStatics.GetPlayerCharacter` 0) (`self.Distance`))))

(event `Random Roam`
  (`|AIMoveTo` self (`NavigationSystemV1.K2_GetRandomReachablePointInRadius` (`self.K2_GetActorLocation`) (`self.MaxDistance`) null null) null 1.0
    (:`OnSuccess`
      (`self.Random Roam`))))

(event `self.ReceiveBeginPlay`
  (set `CharacterMovementComponent.MaxWalkSpeed` (`self.MaxSpeed`) (`self.CharacterMovement`))
  (`self.Random Roam`))

(fn `UserConstructionScript`)