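; Coyote time component for a BP_Controller_Game owner, flagging a short grace window for jumping after leaving the ground.
; Each tick it accumulates a timer while the controller is airborne with all jumps remaining, zeroing it otherwise.
; CanBeUsed is true while that timer is non-zero and within CoyoteTimeAcceptance.
; ResetTimer closes the window early by pushing the timer to a large value.
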(event `self.ReceiveBeginPlay`
  (bind _asbp_controller_game (cast `/Game/_GameManager/Game/BP_Controller_Game` (`self.GetOwner`)))
  (set `self.Controller` _asbp_controller_game))

(event `self.ReceiveTick`
  (params (DeltaSeconds :type "Float (single-precision)"))
  (bind _controller (`self.Controller`))
  (bind _controller_2 (`self.Controller`))
  (set `self.Delta` DeltaSeconds)
  (if (and (not (`/Game/_GameManager/Game/BP_Controller_Game.isTouchingGround` (`self.Controller`))) (== (`/Game/_GameManager/Game/BP_Controller_Game.JumpRemaining` _controller) (`/Game/_GameManager/Game/BP_Controller_Game.JumpNumber` _controller)))
    (set `self.Timer` (+ (`self.Timer`) (`self.Delta`)))
    (else
      (set `self.Timer` 0.0)))
  (set `self.CanBeUsed` (and (!= (`self.Timer`) 0.0) (<= (`self.Timer`) (`self.CoyoteTimeAcceptance`)) (== (`/Game/_GameManager/Game/BP_Controller_Game.JumpNumber` _controller_2) (`/Game/_GameManager/Game/BP_Controller_Game.JumpRemaining` _controller_2)))))

(fn `ResetTimer`
  (set `self.Timer` 999.0))