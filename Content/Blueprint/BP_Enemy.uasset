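; BP_Enemy is an enemy that turns toward the player and damages them in timed attack windows.
; Three overlap volumes set flags for focus, attack range and death range, without checking which actor overlapped.
; Each Tick, an attack-range timer cycles between attack and cooldown, showing the Arrow and applying damage every frame while attacking with death range occupied.
; While focus is active, the Plane smoothly yaws toward the player via RInterpTo.
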(event `self.ReceiveTick`
  (params (DeltaSeconds :type "Float (single-precision)"))
  (bind _arrow (`self.Arrow`))
  ;[0.2941 0.1138 1] Attack and rotate
  (`parent.ReceiveTick` DeltaSeconds)
  (`|ExecutionSequence`
    (:`then_0`
      (bind _isready (`self.CheckAttackCoolDown`))
      (if _isready
        (if (`self.IsPlayerInDeathRange`)
          (`GameplayStatics.ApplyDamage` (`GameplayStatics.GetPlayerCharacter` 0) 10.0))
        (`SceneComponent.SetVisibility` _arrow true false)
        (else
          (`SceneComponent.SetVisibility` _arrow false false))))
    (:`then_1`
      (`self.RotateTowardsPlayer`))))

(event `self.ReceiveBeginPlay`
  ;[0.3279 1 0.2965] Base Blueprint
  (`parent.ReceiveBeginPlay`)
  (`SceneComponent.SetVisibility` (`self.Arrow`) false false))

(event `self.FocusDetection.OnComponentBeginOverlap`
  (params (OverlappedComponent :type "PrimitiveComponent Object Reference") (OtherActor :type "Actor Object Reference") (OtherComp :type "PrimitiveComponent Object Reference") (OtherBodyIndex :type Integer) (bFromSweep :type Boolean) (SweepResult :type "HitResult Structure (by ref)"))
  ;[1 0.3997 0.9134] Player Detection
  (set `self.IsPlayerDetected` true))

(event `self.AttackDetection.OnComponentBeginOverlap`
  (params (OverlappedComponent :type "PrimitiveComponent Object Reference") (OtherActor :type "Actor Object Reference") (OtherComp :type "PrimitiveComponent Object Reference") (OtherBodyIndex :type Integer) (bFromSweep :type Boolean) (SweepResult :type "HitResult Structure (by ref)"))
  ;[1 0.3997 0.9134] Player Detection
  (set `self.IsPlayerInAttackRange` true))

(event `self.FocusDetection.OnComponentEndOverlap`
  (params (OverlappedComponent :type "PrimitiveComponent Object Reference") (OtherActor :type "Actor Object Reference") (OtherComp :type "PrimitiveComponent Object Reference") (OtherBodyIndex :type Integer))
  ;[1 0.3997 0.9134] Player Detection
  (set `self.IsPlayerDetected` false))

(event `self.AttackDetection.OnComponentEndOverlap`
  (params (OverlappedComponent :type "PrimitiveComponent Object Reference") (OtherActor :type "Actor Object Reference") (OtherComp :type "PrimitiveComponent Object Reference") (OtherBodyIndex :type Integer))
  ;[1 0.3997 0.9134] Player Detection
  (set `self.IsPlayerInAttackRange` false)
  (set `self.AttackTimer` 0.0)
  (`SceneComponent.SetVisibility` (`self.Arrow`) false true))

(event `self.DeathDetection.OnComponentBeginOverlap`
  (params (OverlappedComponent :type "PrimitiveComponent Object Reference") (OtherActor :type "Actor Object Reference") (OtherComp :type "PrimitiveComponent Object Reference") (OtherBodyIndex :type Integer) (bFromSweep :type Boolean) (SweepResult :type "HitResult Structure (by ref)"))
  ;[1 0.3997 0.9134] Player Detection
  (set `self.IsPlayerInDeathRange` true))

(event `self.DeathDetection.OnComponentEndOverlap`
  (params (OverlappedComponent :type "PrimitiveComponent Object Reference") (OtherActor :type "Actor Object Reference") (OtherComp :type "PrimitiveComponent Object Reference") (OtherBodyIndex :type Integer))
  ;[1 0.3997 0.9134] Player Detection
  (set `self.IsPlayerInDeathRange` false))

(fn `CheckAttackCoolDown`
  (returns (isReady :type Boolean))
  (if (`self.IsPlayerInAttackRange`)
    (bind _output_get (set `self.AttackTimer` (+ (`self.AttackTimer`) (`GameplayStatics.GetWorldDeltaSeconds`))))
    (if (> _output_get (`self.AttackDuration`))
      (if (> (`self.AttackTimer`) (+ (`self.AttackCooldown`) (`self.AttackDuration`)))
        (set `self.AttackTimer` 0.0))
      (return false)
      (else
        (return true)))
    (else
      (return false))))

(fn `FFInteract`
  (`parent.FFInteract`))

(fn `RotateTowardsPlayer`
  (bind _returnvalue_location (`KismetMathLibrary.BreakTransform` (`self.GetTransform` (`GameplayStatics.GetPlayerPawn` 0))))
  (bind (_returnvalue_roll _returnvalue_pitch _returnvalue_yaw) (`KismetMathLibrary.BreakRotator` (`KismetMathLibrary.FindLookAtRotation` (`SceneComponent.K2_GetComponentLocation` (`self.Plane`)) _returnvalue_location)))
  (if (`self.IsPlayerDetected`)
    (`SceneComponent.K2_SetWorldRotation` (`self.Plane`) (`KismetMathLibrary.RInterpTo` (`SceneComponent.K2_GetComponentRotation` (`self.Plane`)) (`KismetMathLibrary.MakeRotator` 90.0 0.0 (+ _returnvalue_yaw 270.0)) (`GameplayStatics.GetWorldDeltaSeconds`) (`self.RotationInterpSpeed`)) false false)))

(fn `UserConstructionScript`
  (`parent.UserConstructionScript`))