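; Platform that sinks from an up pose to a down pose while the player pawn is in its Box trigger, then rises back once they leave.
; Overlap events interrupt the opposite MoveComponentTo on the Cube, with configurable waits and state flags gating each move.
; Travel time scales with remaining distance, keeping reversals consistent.
; The construction script places marker components at both poses.
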(event `self.ReceiveBeginPlay`
  (bind _cube (`self.Cube`))
  (bind (_returnvalue_x _returnvalue_y _returnvalue_z) (`KismetMathLibrary.BreakVector` (`KismetMathLibrary.TransformLocation` (`self.UpPos`))))
  (bind (_relativelocation_x _relativelocation_y) (`KismetMathLibrary.BreakVector` (`SceneComponent.RelativeLocation` _cube)))
  ;[0.07573 0.3843 1] Setup Position to Up Pose
  (`SceneComponent.K2_SetRelativeLocation` _cube (`KismetMathLibrary.MakeVector` _relativelocation_x _relativelocation_y _returnvalue_z) false false)
  (set `self.IsOnTop` true))

(event `self.Box.OnComponentBeginOverlap`
  (params (OverlappedComponent :type "PrimitiveComponent Object Reference") (OtherActor :type "Actor Object Reference") (OtherComp :type "PrimitiveComponent Object Reference") (OtherBodyIndex :type Integer) (bFromSweep :type Boolean) (SweepResult :type "HitResult Structure (by ref)"))
  (bind _cube (`self.Cube`))
  (bind _ease (`self.Ease`))
  (bind _cube_2 (`self.Cube`))
  (bind _ease_2 (`self.Ease`))
  (bind (_returnvalue_x _returnvalue_y _returnvalue_z) (`KismetMathLibrary.BreakVector` (`KismetMathLibrary.TransformLocation` (`self.UpPos`))))
  (bind (_returnvalue_x_2 _returnvalue_y_2 _returnvalue_z_2) (`KismetMathLibrary.BreakVector` (`KismetMathLibrary.TransformLocation` (`self.DownPos`))))
  (bind (_relativelocation_x _relativelocation_y) (`KismetMathLibrary.BreakVector` (`SceneComponent.RelativeLocation` _cube)))
  (bind (_relativelocation_x_2 _relativelocation_y_2) (`KismetMathLibrary.BreakVector` (`SceneComponent.RelativeLocation` _cube_2)))
  (if (== OtherActor (`GameplayStatics.GetPlayerPawn` 0))
    (`|ExecutionSequence`
      (:`then_0`
        (`self.SetDownSpeed`))
      (:`then_1`
        (goto _label_3 :!via `Stop`))
      (:`then_2`
        (set `self.IsMovingDown` true)
        (set `self.IsMovingUp` false))
      (:`then_3`
        (if (`self.IsMovingUp`)
          _
          (elif (`self.IsOnTop`)
            (`KismetSystemLibrary.Delay` (`self.WaitTopTime`))
            (if (not (`self.IsMovingUp`))
              (set `self.IsOnTop` false :!label _label)
              ;[1 0.6445 0.3763] Move to the bottom
              (`KismetSystemLibrary.MoveComponentTo` _cube (`KismetMathLibrary.MakeVector` _relativelocation_x _relativelocation_y _returnvalue_z_2) (`SceneComponent.RelativeRotation` _cube) _ease _ease (`self.CurrentDownSpeed`) :!label _label_2))
            (else
              (goto _label))))))))

(event `self.Box.OnComponentEndOverlap`
  (params (OverlappedComponent :type "PrimitiveComponent Object Reference") (OtherActor :type "Actor Object Reference") (OtherComp :type "PrimitiveComponent Object Reference") (OtherBodyIndex :type Integer))
  (bind _cube (`self.Cube`))
  (bind _ease (`self.Ease`))
  (bind (_returnvalue_x _returnvalue_y _returnvalue_z) (`KismetMathLibrary.BreakVector` (`KismetMathLibrary.TransformLocation` (`self.UpPos`))))
  (bind (_relativelocation_x _relativelocation_y) (`KismetMathLibrary.BreakVector` (`SceneComponent.RelativeLocation` _cube)))
  (if (== OtherActor (`GameplayStatics.GetPlayerPawn` 0))
    (`|ExecutionSequence`
      (:`then_0`
        (`self.SetUpSpeed`))
      (:`then_1`
        (goto _label_2 :!via `Stop`))
      (:`then_2`
        (set `self.IsMovingDown` false)
        (set `self.IsMovingUp` true))
      (:`then_3`
        (`KismetSystemLibrary.Delay` (`self.WaitBottomTime`))
        (if (not (`self.IsMovingDown`))
          ;[1 0.6445 0.3763] Move to the top
          (`KismetSystemLibrary.MoveComponentTo` _cube (`KismetMathLibrary.MakeVector` _relativelocation_x _relativelocation_y _returnvalue_z) (`SceneComponent.RelativeRotation` _cube) _ease _ease (`self.CurrentUpSpeed`) :!label _label_3)
          (set `self.IsOnTop` true))))))

(fn `SetDownSpeed`
  (bind (_returnvalue_x _returnvalue_y _returnvalue_z) (`KismetMathLibrary.BreakVector` (`KismetMathLibrary.TransformLocation` (`self.DownPos`))))
  (bind (_returnvalue_x_2 _returnvalue_y_2 _returnvalue_z_2) (`KismetMathLibrary.BreakVector` (`KismetMathLibrary.TransformLocation` (`self.DownPos`))))
  (bind (_returnvalue_x_3 _returnvalue_y_3 _returnvalue_z_3) (`KismetMathLibrary.BreakVector` (`KismetMathLibrary.TransformLocation` (`self.UpPos`))))
  (bind (_relativelocation_x _relativelocation_y _relativelocation_z) (`KismetMathLibrary.BreakVector` (`SceneComponent.RelativeLocation` (`self.Cube`))))
  (set `self.CurrentDownSpeed` (/ (* (- _relativelocation_z _returnvalue_z) (`self.DownSpeed`)) (- _returnvalue_z_3 _returnvalue_z_2))))

(fn `SetUpSpeed`
  (bind (_returnvalue_x _returnvalue_y _returnvalue_z) (`KismetMathLibrary.BreakVector` (`KismetMathLibrary.TransformLocation` (`self.UpPos`))))
  (bind (_returnvalue_x_2 _returnvalue_y_2 _returnvalue_z_2) (`KismetMathLibrary.BreakVector` (`KismetMathLibrary.TransformLocation` (`self.UpPos`))))
  (bind (_returnvalue_x_3 _returnvalue_y_3 _returnvalue_z_3) (`KismetMathLibrary.BreakVector` (`KismetMathLibrary.TransformLocation` (`self.DownPos`))))
  (bind (_relativelocation_x _relativelocation_y _relativelocation_z) (`KismetMathLibrary.BreakVector` (`SceneComponent.RelativeLocation` (`self.Cube`))))
  (set `self.CurrentUpSpeed` (/ (* (- _relativelocation_z _returnvalue_z) (`self.UpSpeed`)) (- _returnvalue_z_3 _returnvalue_z_2))))

(fn `UserConstructionScript`
  (`SceneComponent.K2_SetRelativeTransform` (`self.UpPosAsset`) (`self.UpPos`) false false)
  (`SceneComponent.K2_SetRelativeTransform` (`self.DownPosAsset`) (`self.DownPos`) false false))