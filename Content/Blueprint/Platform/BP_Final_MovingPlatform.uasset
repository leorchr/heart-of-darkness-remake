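; BP_Final_MovingPlatform is a moving platform that starts when the player pawn overlaps its Box while it is not already moving.
; Move slides Cube to EndPos over InterpSpeed seconds with optional easing, clearing IsMoving only on completion.
; Reset stops the move and snaps Cube to StartPos, without clearing IsMoving itself.
; The construction script places StartPosAsset and EndPosAsset at the two endpoint transforms.
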(event `Move`
  (bind _ease (`self.Ease`))
  (bind _cube (`self.Cube`))
  (set `self.isMoving` true)
  (`KismetSystemLibrary.MoveComponentTo` _cube (`KismetMathLibrary.TransformLocation` (`self.EndPos`)) (`SceneComponent.RelativeRotation` _cube) _ease _ease (`self.InterpSpeed`) :!label _label)
  (set `self.isMoving` false))

(event `Reset`
  (bind _cube (`self.Cube`))
  (`|ExecutionSequence`
    (:`then_0`
      (goto _label :!via `Stop`))
    (:`then_1`
      (`KismetSystemLibrary.MoveComponentTo` _cube (`KismetMathLibrary.TransformLocation` (`self.StartPos`)) (`SceneComponent.RelativeRotation` _cube) false false 0.0))))

(event `self.Box.OnComponentBeginOverlap`
  (params (OverlappedComponent :type "PrimitiveComponent Object Reference") (OtherActor :type "Actor Object Reference") (OtherComp :type "PrimitiveComponent Object Reference") (OtherBodyIndex :type Integer) (bFromSweep :type Boolean) (SweepResult :type "HitResult Structure (by ref)"))
  (if (and (== OtherActor (`GameplayStatics.GetPlayerPawn` 0)) (not (`self.isMoving`)))
    (`self.Move`)))

(fn `UserConstructionScript`
  (`SceneComponent.K2_SetRelativeTransform` (`self.StartPosAsset`) (`self.StartPos`) false false)
  (`SceneComponent.K2_SetRelativeTransform` (`self.EndPosAsset`) (`self.EndPos`) false false))