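; BP_Checkpoint is a checkpoint actor that updates the player's respawn point when the game character enters its trigger.
; On overlap it registers itself as LastCheckpoint on BP_GM_Game, then calls SetNewSpawn on the character.
; The spawn transform comes from the POS component, with yaw offset by 90 degrees and unit scale.
; A PlaySound2D node is present but unconnected.
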(event `self.Trigger.OnComponentBeginOverlap`
  (params (OverlappedComponent :type "PrimitiveComponent Object Reference") (OtherActor :type "Actor Object Reference") (OtherComp :type "PrimitiveComponent Object Reference") (OtherBodyIndex :type Integer) (bFromSweep :type Boolean) (SweepResult :type "HitResult Structure (by ref)"))
  (bind (_returnvalue_location _returnvalue_rotation) (`KismetMathLibrary.BreakTransform` (`SceneComponent.K2_GetComponentToWorld` (`self.POS`))))
  (bind _asbp_character_game (cast `/Game/_GameManager/Game/BP_Character_Game` OtherActor))
  (bind _asbp_gm_game (cast `/Game/_GameManager/Game/BP_GM_Game` (`GameplayStatics.GetGameMode`)))
  (set `/Game/_GameManager/Game/BP_GM_Game.Last Checkpoint` self _asbp_gm_game)
  (`/Game/_GameManager/Game/BP_Character_Game.SetNewSpawn` _asbp_character_game (`KismetMathLibrary.MakeTransform` _returnvalue_location (`KismetMathLibrary.MakeRotator` (.roll _returnvalue_rotation) (.pitch _returnvalue_rotation) (+ (.yaw _returnvalue_rotation) 90.0)))))

(fn `UserConstructionScript`)