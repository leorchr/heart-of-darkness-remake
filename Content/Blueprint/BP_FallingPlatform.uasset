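; Falling platform that drops after the player steps on it, then rises back to its top position after a delay.
; Box overlap flags the player as on-platform in the game controller, refills jumps, swaps the cube's material and starts the fall timer.
; Timers chain eased MoveComponentTo moves between UpPos and DownPos, re-triggering if the player is still aboard after reset.
; The construction script places marker components at both poses.
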(event `self.ReceiveBeginPlay`
  (bind _cube (`self.Cube`))
  (bind (_returnvalue_x _returnvalue_y _returnvalue_z) (`KismetMathLibrary.BreakVector` (`KismetMathLibrary.TransformLocation` (`self.UpPos`))))
  (bind (_relativelocation_x _relativelocation_y) (`KismetMathLibrary.BreakVector` (`SceneComponent.RelativeLocation` _cube)))
  ;[0.07573 0.3843 1] Setup Position to Up Pose
  (`SceneComponent.K2_SetRelativeLocation` _cube (`KismetMathLibrary.MakeVector` _relativelocation_x _relativelocation_y _returnvalue_z) false false)
  (bind _asbp_controller_game (cast `/Game/_GameManager/Game/BP_Controller_Game` (`GameplayStatics.GetPlayerController` 0)))
  (set `self.Controller` _asbp_controller_game))

(event `Elevate`
  (bind _cube (`self.Cube`))
  (bind _ease (`self.Ease`))
  (bind (_returnvalue_x _returnvalue_y _returnvalue_z) (`KismetMathLibrary.BreakVector` (`KismetMathLibrary.TransformLocation` (`self.UpPos`))))
  (bind (_relativelocation_x _relativelocation_y) (`KismetMathLibrary.BreakVector` (`SceneComponent.RelativeLocation` _cube)))
  ;[1 0.6445 0.3763] Move to the top
  (`KismetSystemLibrary.MoveComponentTo` _cube (`KismetMathLibrary.MakeVector` _relativelocation_x _relativelocation_y _returnvalue_z) (`SceneComponent.RelativeRotation` _cube) _ease _ease (`self.UpSpeed`))
  (set `self.inProgress` false)
  (`PrimitiveComponent.SetMaterial` (`self.Cube`) 0 "/Engine/EngineMaterials/WorldGridMaterial.WorldGridMaterial")
  ;[1 0.3095 0.3613] Player Enter Platform
  (if (and (not (`self.inProgress`)) (`/Game/_GameManager/Game/BP_Controller_Game.isOnPlatform` (`self.Controller`))) :!label _label
    (set `self.inProgress` true)
    (`PrimitiveComponent.SetMaterial` (`self.Cube`) 0 "/Engine/MapTemplates/Materials/BasicAsset01.BasicAsset01")
    (`KismetSystemLibrary.K2_SetTimerDelegate` (delegate `Falling`) (`self.TimeBeforeFalling`))))

(event `Falling`
  (bind _cube (`self.Cube`))
  (bind _ease (`self.Ease`))
  (bind (_returnvalue_x _returnvalue_y _returnvalue_z) (`KismetMathLibrary.BreakVector` (`KismetMathLibrary.TransformLocation` (`self.DownPos`))))
  (bind (_relativelocation_x _relativelocation_y) (`KismetMathLibrary.BreakVector` (`SceneComponent.RelativeLocation` _cube)))
  ;[1 0.6445 0.3763] Move to the bottom
  (`KismetSystemLibrary.MoveComponentTo` _cube (`KismetMathLibrary.MakeVector` _relativelocation_x _relativelocation_y _returnvalue_z) (`SceneComponent.RelativeRotation` _cube) _ease _ease (`self.DownSpeed`))
  (`KismetSystemLibrary.K2_SetTimerDelegate` (delegate `Elevate`) (`self.TimeBeforeReset`)))

(event `self.Box.OnComponentBeginOverlap`
  (params (OverlappedComponent :type "PrimitiveComponent Object Reference") (OtherActor :type "Actor Object Reference") (OtherComp :type "PrimitiveComponent Object Reference") (OtherBodyIndex :type Integer) (bFromSweep :type Boolean) (SweepResult :type "HitResult Structure (by ref)"))
  (bind _controller (`self.Controller`))
  ;[1 0.3095 0.3613] Player Enter Platform
  (if (== OtherActor (`GameplayStatics.GetPlayerPawn` 0))
    (`|ExecutionSequence`
      (:`then_0`
        (set `/Game/_GameManager/Game/BP_Controller_Game.isOnPlatform` true _controller)
        (set `/Game/_GameManager/Game/BP_Controller_Game.JumpRemaining` 2 _controller))
      (:`then_1`
        (goto _label)))))

(event `self.Box.OnComponentEndOverlap`
  (params (OverlappedComponent :type "PrimitiveComponent Object Reference") (OtherActor :type "Actor Object Reference") (OtherComp :type "PrimitiveComponent Object Reference") (OtherBodyIndex :type Integer))
  ;[1 0.3095 0.3613] Player Exit Platform
  (if (== OtherActor (`GameplayStatics.GetPlayerPawn` 0))
    (set `/Game/_GameManager/Game/BP_Controller_Game.isOnPlatform` false (`self.Controller`))))

(fn `SetDownSpeed`
  (bind (_returnvalue_x _returnvalue_y _returnvalue_z) (`KismetMathLibrary.BreakVector` (`KismetMathLibrary.TransformLocation` (`self.DownPos`))))
  (bind (_returnvalue_x_2 _returnvalue_y_2 _returnvalue_z_2) (`KismetMathLibrary.BreakVector` (`KismetMathLibrary.TransformLocation` (`self.DownPos`))))
  (bind (_returnvalue_x_3 _returnvalue_y_3 _returnvalue_z_3) (`KismetMathLibrary.BreakVector` (`KismetMathLibrary.TransformLocation` (`self.UpPos`))))
  (bind (_relativelocation_x _relativelocation_y _relativelocation_z) (`KismetMathLibrary.BreakVector` (`SceneComponent.RelativeLocation` (`self.Cube`))))
  (set `self.DownSpeed` (/ (* (- _relativelocation_z _returnvalue_z) 0.0) (- _returnvalue_z_3 _returnvalue_z_2))))

(fn `SetUpSpeed`
  (bind (_returnvalue_x _returnvalue_y _returnvalue_z) (`KismetMathLibrary.BreakVector` (`KismetMathLibrary.TransformLocation` (`self.UpPos`))))
  (bind (_returnvalue_x_2 _returnvalue_y_2 _returnvalue_z_2) (`KismetMathLibrary.BreakVector` (`KismetMathLibrary.TransformLocation` (`self.UpPos`))))
  (bind (_returnvalue_x_3 _returnvalue_y_3 _returnvalue_z_3) (`KismetMathLibrary.BreakVector` (`KismetMathLibrary.TransformLocation` (`self.DownPos`))))
  (bind (_relativelocation_x _relativelocation_y _relativelocation_z) (`KismetMathLibrary.BreakVector` (`SceneComponent.RelativeLocation` (`self.Cube`))))
  (set `self.UpSpeed` (/ (* (- _relativelocation_z _returnvalue_z) 0.0) (- _returnvalue_z_3 _returnvalue_z_2))))

(fn `UserConstructionScript`
  (`SceneComponent.K2_SetRelativeTransform` (`self.UpPosAsset`) (`self.UpPos`) false false)
  (`SceneComponent.K2_SetRelativeTransform` (`self.DownPosAsset`) (`self.DownPos`) false false))