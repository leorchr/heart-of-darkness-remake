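; Trigger volume that shows a tutorial while the player character stands inside its box.
; On overlap begin it asks BP_GM_Game to play the tutorial with its own text lines and icons.
; On overlap end it plays the game mode tutorial widget's fade-out animation, waits briefly, then ends the tutorial.
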(event `self.BoxTuto.OnComponentBeginOverlap`
  (params (OverlappedComponent :type "PrimitiveComponent Object Reference") (OtherActor :type "Actor Object Reference") (OtherComp :type "PrimitiveComponent Object Reference") (OtherBodyIndex :type Integer) (bFromSweep :type Boolean) (SweepResult :type "HitResult Structure (by ref)"))
  (cast `/Game/Player/BP_Character_Game` OtherActor)
  (bind _asbp_gm_game (cast `/Game/_GameManager/Game/BP_GM_Game` (`GameplayStatics.GetGameMode`)))
  (`/Game/_GameManager/Game/BP_GM_Game.Play Tutorial` _asbp_gm_game (`self.Text01`) (`self.Text02`) (`self.Text03`) (`self.Icon`) (`self.Icon02`)))

(event `self.BoxTuto.OnComponentEndOverlap`
  (params (OverlappedComponent :type "PrimitiveComponent Object Reference") (OtherActor :type "Actor Object Reference") (OtherComp :type "PrimitiveComponent Object Reference") (OtherBodyIndex :type Integer))
  (cast `/Game/Player/BP_Character_Game` OtherActor)
  (bind _asbp_gm_game (cast `/Game/_GameManager/Game/BP_GM_Game` (`GameplayStatics.GetGameMode`)))
  (bind _tuto (`/Game/_GameManager/Game/BP_GM_Game.Tuto` _asbp_gm_game))
  (`UserWidget.PlayAnimation` _tuto (`/Game/UI/Tutorial/W_Tutorial.FadeOut` _tuto) 0.0 1 "Forward" 1.0 false)
  (`KismetSystemLibrary.Delay` 0.5)
  (`/Game/_GameManager/Game/BP_GM_Game.End Tutorial` _asbp_gm_game))

(fn `UserConstructionScript`)