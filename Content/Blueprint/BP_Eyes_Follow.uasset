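; BP_Eyes_Follow is an interactable actor, named for following eyes, that fades out and destroys itself once interacted with.
; Its FFInteract override runs the parent logic, sets IsFading and starts a looping timer, guarded by a handle check against duplicates.
; The Fade event, the apparent timer target, steps FadeAlpha down to zero and then destroys the actor.
; No eye-following logic or visual use of FadeAlpha appears in these graphs.
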(event `Fade`
  (bind _output_get (set `self.FadeAlpha` (`KismetMathLibrary.FClamp` (- (`self.FadeAlpha`) 0.05))))
  (if (== _output_get 0.0)
    (`self.K2_DestroyActor`)))

(fn `FFInteract`
  (`parent.FFInteract`)
  (set `self.isFading` true)
  (if (not (`KismetSystemLibrary.K2_IsValidTimerHandle` (`self.eventTH`)))
    (bind _returnvalue (`KismetSystemLibrary.K2_SetTimerDelegate` (`|CreateDelegate` :!event `Fade`) 0.05 true))
    (set `self.eventTH` _returnvalue)))

(fn `UserConstructionScript`
  (`parent.UserConstructionScript`))