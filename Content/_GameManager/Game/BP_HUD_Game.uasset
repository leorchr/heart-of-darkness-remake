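; BP_HUD_Game is the in-game HUD Blueprint that owns the pause menu and switches the game between paused and running.
; On BeginPlay it creates W_PauseMenu once and keeps it hidden in the viewport.
; PauseGame and ResumeGame toggle that widget's visibility and activation, the mouse cursor, the UI-only or game-only input mode, and the global pause state for player 0.
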(event `self.ReceiveBeginPlay`
  ;[1 0.016 0.6654] Create Pause Menu at begining
  (bind _returnvalue (`|CreateWidget` "/Game/UI/InGame/W_PauseMenu.W_PauseMenu_C" (`GameplayStatics.GetPlayerController` 0)))
  (bind _output_get (set `self.PauseMenu` _returnvalue))
  (`UserWidget.AddToViewport` _output_get 0)
  (`Widget.SetVisibility` _output_get "Hidden"))

(event `PauseGame`
  (bind _returnvalue (`GameplayStatics.GetPlayerController` 0))
  (bind _pausemenu (`self.PauseMenu`))
  ;[1 0.016 0.6654] Pause Game
  (set `PlayerController.bShowMouseCursor` true _returnvalue)
  (`WidgetBlueprintLibrary.SetInputMode_UIOnlyEx` _returnvalue _pausemenu)
  (`Widget.SetVisibility` _pausemenu "Visible")
  (`/Game/UI/InGame/W_PauseMenu.ActivatePauseButton` (`self.PauseMenu`))
  (`GameplayStatics.SetGamePaused` true))

(event `ResumeGame`
  (bind _returnvalue (`GameplayStatics.GetPlayerController` 0))
  (bind _pausemenu (`self.PauseMenu`))
  ;[1 0.016 0.6654] Unpause Game
  (set `PlayerController.bShowMouseCursor` false _returnvalue)
  (`WidgetBlueprintLibrary.SetInputMode_GameOnly` _returnvalue)
  (`CommonActivatableWidget.DeactivateWidget` _pausemenu)
  (`Widget.SetVisibility` _pausemenu "Hidden")
  (`GameplayStatics.SetGamePaused` false))

(fn `UserConstructionScript`)