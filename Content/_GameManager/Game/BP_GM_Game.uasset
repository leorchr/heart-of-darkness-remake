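; BP_GM_Game is the game manager that handles the opening cinematic, player respawning and tutorial popups.
; On BeginPlay it plays the intro sequence as a camera animation through the GameplayCamerasSubsystem.
; RespawnPlayer waits briefly, moves the character to the last checkpoint or a PlayerStart fallback, re-enables input, then restores health and resets the player.
; PlayTutorial shows a fading W_Tutorial widget with given texts and icon, which EndTutorial removes.
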(event `self.ReceiveBeginPlay`
  (`self.Play Cinematic` (`self.Cinematic Begin`)))

(event `Respawn Player`
  (params (SpawnTransform :type "Transform Structure"))
  (bind _returnvalue (`GameplayStatics.GetPlayerController` 0))
  (`KismetSystemLibrary.Delay` 1.2)
  (bind _last_checkpoint (`self.last Checkpoint`)
    (:`then`
      (bind _returnvalue_location (`KismetMathLibrary.BreakTransform` (`SceneComponent.K2_GetComponentToWorld` (`/Game/Blueprint/WinLoseCondition/BP_Checkpoint.POS` _last_checkpoint))))
      (`self.K2_SetActorLocation` (`GameplayStatics.GetPlayerCharacter` 0) _returnvalue_location false false))
    (:`else`
      (bind _returnvalue_2 (`GameplayStatics.GetActorOfClass` "/Script/Engine.PlayerStart"))
      (`self.K2_SetActorLocation` (`GameplayStatics.GetPlayerCharacter` 0) (`self.K2_GetActorLocation` _returnvalue_2) false false)))
  (`self.EnableInput` _returnvalue _returnvalue)
  (bind _asbp_character_game (cast `/Game/Player/BP_Character_Game` (`GameplayStatics.GetPlayerCharacter` 0)))
  (set `/Game/Player/BP_Character_Game.Health` (`/Game/Player/BP_Character_Game.maxHealth` _asbp_character_game) _asbp_character_game)
  (`/Game/Player/BP_Character_Game.resetPlayer` _asbp_character_game))

(fn `End Tutorial`
  (`Widget.RemoveFromParent` (`self.Tuto`)))

(fn `Play Cinematic`
  (params (Sequence :type "CameraAnimationSequence Object Reference"))
  (`GameplayCamerasSubsystem.PlayCameraAnimation` :`self` (subsystem `GameplayCamerasSubsystem`) :`PlayerController` (`GameplayStatics.GetPlayerController` 0) :`Sequence` Sequence))

(fn `Play Tutorial`
  (params (Text01 :type Text) (Text02 :type Text) (Icon :type "SlateBrush Structure"))
  (bind _returnvalue (`|CreateWidget` "/Game/UI/Tutorial/W_Tutorial.W_Tutorial_C" (`GameplayStatics.GetPlayerController` 0)))
  (bind _output_get (set `self.Tuto` _returnvalue))
  (set `/Game/UI/Tutorial/W_Tutorial.Text01` Text01 _returnvalue)
  (set `/Game/UI/Tutorial/W_Tutorial.Text02` Text02 _returnvalue)
  (set `/Game/UI/Tutorial/W_Tutorial.IconBrush` Icon _returnvalue)
  (`UserWidget.AddToViewport` _output_get 0)
  (`UserWidget.PlayAnimation` _output_get (`/Game/UI/Tutorial/W_Tutorial.FadeIn` _returnvalue) 0.0 1 "Forward" 1.0 false))

(fn `UserConstructionScript`)