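; Player controller that turns Enhanced Input into BP_Character_Game movement, camera look, sprint, aiming, firefly shooting and pause.
; A looping timer runs arrow line traces to detect ground and refill multi-jumps, launched by movement state with coyote support.
; Aiming blocks jump and sprint and enables rate-limited projectiles aimed by camera trace, which also drives arm animation rotation.
; Look sensitivity loads from save and scales over interactables for aim magnetism.
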(event Custom|Event%20Check%20Ground
  (CallFunction|CheckGround))

(event Input|EnhancedActionEvents|EnhancedInputActionIA_Move
  (params (ActionValue :type Vector%202D%20Structure) (ElapsedSeconds :type Float%20%28double-precision%29) (TriggeredSeconds :type Float%20%28double-precision%29) (InputAction :type Input%20Action%20Object%20Reference :default "/Game/_GameManager/Input/Actions/IA_Move.IA_Move"))
  (bind (_x _y) (Math|Vector2D|BreakVector2D ActionValue))
  (bind _characterbp (Variables|Default|GetCharacterBP))
  (bind _camera (Variables|/Game/Player/BP_Character_Game.BP_Character_Game_C|GetCamera _characterbp))
  (bind _returnvalue (Transformation|GetWorldRotation _camera))
  (bind _returnvalue_2 (Math|Rotator|MakeRotator (.roll _returnvalue) 0.0 (.yaw _returnvalue)))
  (bind _returnvalue_3 (Math|Vector|GetRightVector _returnvalue_2))
  (bind _returnvalue_4 (Math|Vector|GetForwardVector _returnvalue_2))
  (:Triggered
    (Pawn|Input|AddMovementInput _characterbp _returnvalue_4 _y false)
    (Pawn|Input|AddMovementInput _characterbp _returnvalue_3 _x false)
    (Variables|Default|SetTargetRotation (Math|Rotator|MakeRotator 0.0 0.0 (+ (.Yaw (Math|Rotator|BreakRotator (CallFunction|CalculateCharacterRotationTarget ActionValue _returnvalue_4 _returnvalue_3))) -9e+01)))))

(event Input|EnhancedActionEvents|EnhancedInputActionIA_Look
  (params (ActionValue :type Vector%202D%20Structure) (ElapsedSeconds :type Float%20%28double-precision%29) (TriggeredSeconds :type Float%20%28double-precision%29) (InputAction :type Input%20Action%20Object%20Reference :default "/Game/_GameManager/Input/Actions/IA_Look.IA_Look"))
  (bind _aimmultiplier (CallFunction|EnemyIsinCrosshair))
  (bind _camerasensitivity (Variables|Camera|GetCameraSensitivity))
  (bind _characterbp (Variables|Default|GetCharacterBP))
  (bind _camangleclampy (Variables|Camera|GetCamAngleClampY))
  (bind _currentcam (Variables|/Game/Player/BP_Character_Game.BP_Character_Game_C|GetcurrentCam _characterbp))
  (bind _springarm (Variables|/Game/Player/BP_Character_Game.BP_Character_Game_C|GetSpringArm _characterbp))
  (bind _sensitivitymultiplier (Utilities|Struct|BreakSCamType _currentcam))
  (bind _returnvalue (Transformation|GetWorldRotation _springarm))
  (bind _returnvalue_2 (* ActionValue _camerasensitivity _sensitivitymultiplier _aimmultiplier))
  (bind (_x _y) (Math|Vector2D|BreakVector2D _returnvalue_2))
  (:Triggered
    (Variables|/Game/Player/BP_Character_Game.BP_Character_Game_C|SetTargetArmRotation _characterbp (Math|Rotator|MakeRotator 0.0 (Math|Float|ClampAngle (- (.pitch _returnvalue) _y) (.x _camangleclampy) (.y _camangleclampy)) (+ (.yaw _returnvalue) _x)))))

(event Input|EnhancedActionEvents|EnhancedInputActionIA_Sprint
  (params (ActionValue :type Boolean) (ElapsedSeconds :type Float%20%28double-precision%29) (TriggeredSeconds :type Float%20%28double-precision%29) (InputAction :type Input%20Action%20Object%20Reference :default "/Game/_GameManager/Input/Actions/IA_Sprint.IA_Sprint"))
  ;[0.2232 0.117 1] Sprint Behaviour
  (:Triggered
    (CallFunction|StartRunning))
  (:Canceled
    (CallFunction|StopRunning :!label _label))
  (:Completed
    (goto _label)))

(event Input|EnhancedActionEvents|EnhancedInputActionIA_Jump
  (params (ActionValue :type Boolean) (ElapsedSeconds :type Float%20%28double-precision%29) (TriggeredSeconds :type Float%20%28double-precision%29) (InputAction :type Input%20Action%20Object%20Reference :default "/Game/_GameManager/Input/Actions/IA_Jump.IA_Jump"))
  (:Started
    (bind _canjump (CallFunction|CheckCanJump))
    (if _canjump
      (CallFunction|Jump))))

(event Input|EnhancedActionEvents|EnhancedInputActionIA_CamReset
  (params (ActionValue :type Boolean) (ElapsedSeconds :type Float%20%28double-precision%29) (TriggeredSeconds :type Float%20%28double-precision%29) (InputAction :type Input%20Action%20Object%20Reference :default "/Game/_GameManager/Input/Actions/IA_CamReset.IA_CamReset"))
  (:Started
    (Default|RecentrateCam (Variables|Default|GetCharacterBP))))

(event Input|EnhancedActionEvents|EnhancedInputActionIA_Aim
  (params (ActionValue :type Boolean) (ElapsedSeconds :type Float%20%28double-precision%29) (TriggeredSeconds :type Float%20%28double-precision%29) (InputAction :type Input%20Action%20Object%20Reference :default "/Game/_GameManager/Input/Actions/IA_Aim.IA_Aim"))
  (bind _characterbp (Variables|Default|GetCharacterBP))
  (bind _characterbp_2 (Variables|Default|GetCharacterBP))
  (bind _crosshair (Variables|Default|GetCrossHair))
  (bind _charactermovement (Variables|/Script/Engine.Character|GetCharacterMovement _characterbp_2))
  (:Triggered
    (if (and (not (Variables|Default|GetisAiming)) (Variables|Default|GetisTouchingGround))
      (if (Variables|Default|GethasAbilityShoot) :!label _label
        (Default|Aim _characterbp true)
        (Variables|Default|SetisAiming true)
        (Default|VisibleCrosshair _crosshair)
        ;[0.8095 0.01179 1] Disable Running when aiming
        (CallFunction|StopRunning)
        (Variables|Character|SetcanRun false)
        (Variables|/Script/Engine.CharacterMovementComponent|SetMaxWalkSpeed _charactermovement (Variables|Character|GetmaxAimingSpeed)))))
  (:Started
    (if (Variables|Default|GetisTouchingGround)
      (goto _label)))
  (:Canceled
    (Default|Aim _characterbp false :!label _label_2)
    (Variables|Default|SetisAiming false)
    (Default|UnvisibleCrosshair _crosshair)
    (Variables|Character|SetcanRun true)
    (Variables|/Script/Engine.CharacterMovementComponent|SetMaxWalkSpeed _charactermovement (Variables|Character|GetmaxWalkingSpeed)))
  (:Completed
    (goto _label_2)))

(event Input|EnhancedActionEvents|EnhancedInputActionIA_Pause
  (params (ActionValue :type Boolean) (ElapsedSeconds :type Float%20%28double-precision%29) (TriggeredSeconds :type Float%20%28double-precision%29) (InputAction :type Input%20Action%20Object%20Reference :default "/Game/_GameManager/Input/Actions/IA_Pause.IA_Pause"))
  (bind _returnvalue (HUD|GetHUD))
  ;[0.2232 0.117 1] Open Pause Menu
  (:Started
    (if (Game|IsGamePaused)
      (bind _asbp_hud_game (Utilities|Casting|CastToBP_HUD_Game _returnvalue))
      (Default|ResumeGame _asbp_hud_game)
      (else
        (bind _asbp_hud_game_2 (Utilities|Casting|CastToBP_HUD_Game _returnvalue))
        (Default|PauseGame _asbp_hud_game_2)))))

(event Input|EnhancedActionEvents|EnhancedInputActionIA_FireflyLaunch
  (params (ActionValue :type Boolean) (ElapsedSeconds :type Float%20%28double-precision%29) (TriggeredSeconds :type Float%20%28double-precision%29) (InputAction :type Input%20Action%20Object%20Reference :default "/Game/_GameManager/Input/Actions/IA_FireflyLaunch.IA_FireflyLaunch"))
  (:Started
    (bind _can_ (CallFunction|CanShoot))
    (if _can_
      (CallFunction|Shoot)
      (Default|ShowProgress (Variables|Default|GetCrossHair)))))

(event Input|EnhancedActionEvents|EnhancedInputActionIA_ListInputs
  (params (ActionValue :type Boolean) (ElapsedSeconds :type Float%20%28double-precision%29) (TriggeredSeconds :type Float%20%28double-precision%29) (InputAction :type Input%20Action%20Object%20Reference :default "/Game/_GameManager/Input/Actions/IA_ListInputs.IA_ListInputs"))
  (bind _listinputs (Variables|Default|GetListInputs))
  (:Started
    (if (Variables|Default|GetisListInputs?)
      (Variables|Default|SetisListInputs? false)
      (Widget|SetVisibility _listinputs "Hidden")
      (else
        (Variables|Default|SetisListInputs? true)
        (Widget|SetVisibility _listinputs "Visible")))))

(event EventTick
  (params (DeltaSeconds :type Float%20%28single-precision%29))
  (bind _characterbp (Variables|Default|GetCharacterBP))
  (bind _mesh (Variables|/Script/Engine.Character|GetMesh _characterbp))
  (if (not (Game|IsGamePaused))
    (Variables|Default|SetFireflySTime (Math|Float|Clamp(Float) (+ (Variables|Default|GetFireflySTime) (* DeltaSeconds (Variables|Firefly|GetFireflyShootRate))) -1.0 1.1))
    (Transformation|SetWorldRotation _mesh (Math|Interpolation|RInterpTo (Transformation|GetWorldRotation _mesh) (Variables|Default|GetTargetRotation) 0.1 1.0) false false)
    ;[1 0.1199 0] Compute Aim Point for Arm ABP
    (if (Variables|Default|GetisAiming)
      (CallFunction|GetProjectileTransform))))

(event EventBeginPlay
  (CallFunction|ReloadSensitivity)
  (Input|AddMappingContext (PlayerController|LocalPlayerSubsystems|GetEnhancedInputLocalPlayerSubsystem) "/Game/_GameManager/Input/IMC_Default.IMC_Default" 0 "(bIgnoreAllPressedKeysUntilRelease=True,bForceImmediately=False)")
  (bind _asbp_character_game (Utilities|Casting|CastToBP_Character_Game (Game|GetPlayerCharacter 0)))
  (Variables|Default|SetCharacterBP _asbp_character_game)
  (Input|SetInputModeGameOnly (Game|GetPlayerController 0) false)
  (Utilities|SetVariables
    (:Out
      (Utilities|Time|SetTimerbyFunctionName 0 "Event Check Ground" 0.2 true)
      (bind _returnvalue (UserInterface|CreateWidget "/Game/UI/InGame/W_Crosshair.W_Crosshair_C"))
      (bind _output_get (Variables|Default|SetCrossHair _returnvalue))
      (UserInterface|Viewport|AddtoViewport _output_get 0))))

(event Input|KeyboardEvents|DebugKeyX
  (params (Key :type Key%20Structure :default "None") (ActionValue :type Input%20Action%20Value%20Structure))
  (:Pressed
    (Variables|Default|SethasAbilityShoot (not (Variables|Default|GethasAbilityShoot)))))

(event Input|KeyboardEvents|M
  (params (Key :type Key%20Structure :default "None"))
  (:Pressed
    (Game|Damage|ApplyDamage (Variables|Default|GetCharacterBP) 1e+01 0 0)))

(event Input|KeyboardEvents|V
  (params (Key :type Key%20Structure :default "None"))
  (:Pressed
    (Default|ChangeCamType (Variables|Default|GetCharacterBP) "NewEnumerator0")))

(fn ConstructionScript)

(fn CheckCanJump
  (return (Math|Boolean|ANDBoolean (Math|Boolean|ORBoolean (Variables|Default|GetisTouchingGround) (Variables|/Game/Blueprint/Coyote/BP_Coyote_AC.BP_Coyote_AC_C|GetCanBeUsed (Variables|Default|GetCoyote)) (Variables|Default|GetisOnPlatform) (!= (Variables|Default|GetJumpRemaining) (Variables|Jump|GetJumpNumber))) (> (Variables|Default|GetJumpRemaining) 0) (not (Variables|Default|GetisAiming)))))

(fn CalculateJumpVelocity
  (params (jumpType :type EJumpType%20Enum :default "NewEnumerator3"))
  (bind _targetrotation (Variables|Default|GetTargetRotation))
  (bind _horizontaljumpforce (Variables|Jump|GethorizontalJumpForce))
  (bind _veticaljumpforce (Variables|Jump|GetveticalJumpForce))
  (bind _horizontalzratio (Variables|Jump|GetHorizontalZRatio))
  (bind _returnvalue (* _veticaljumpforce _horizontalzratio))
  (bind _returnvalue_2 (+ (.yaw _targetrotation) 9e+01))
  (bind _returnvalue_3 (Math|Vector|GetForwardVector (Math|Rotator|MakeRotator (.roll _targetrotation) (.pitch _targetrotation) _returnvalue_2)))
  (bind _returnvalue_4 (Math|Vector|Normalize _returnvalue_3))
  (bind _returnvalue_5 (Math|Vector|MakeVector (.x _returnvalue_4) (.y _returnvalue_4) 0.0))
  (bind _returnvalue_6 (* _returnvalue_5 _horizontaljumpforce))
  (bind _returnvalue_7 (Math|Vector|MakeVector (.x _returnvalue_6) (.y _returnvalue_6) _returnvalue))
  (if (Utilities|Enum|Equal(Enum) jumpType "NewEnumerator3")
    ;[0.2923 0.4411 1] Find what type of jump is done
    (if (Math|Vector|VectorIsNearlyZero (Transformation|GetVelocity (Variables|Default|GetCharacterBP)) 2e+02)
      (LocalVariables|SetcurrentJumpT "NewEnumerator0")
      (elif (not (Variables|Default|GetisRunning))
        (LocalVariables|SetcurrentJumpT "NewEnumerator1")
        (else
          (LocalVariables|SetcurrentJumpT "NewEnumerator2"))))
    (else
      (LocalVariables|SetcurrentJumpT jumpType)))
  (return (Math|Vector|SelectVector (Utilities|Select :Index (LocalVariables|GetcurrentJumpT) :NewEnumerator3 "0, 0, 0" :NewEnumerator0 (Math|Vector|MakeVector 0.0 0.0 (Variables|Jump|GetveticalJumpForce)) :NewEnumerator1 _returnvalue_7 :NewEnumerator2 (* _returnvalue_7 (Variables|Jump|GetRunJumpRatio))) (* (Utilities|Select :Index (LocalVariables|GetcurrentJumpT) :NewEnumerator3 "0, 0, 0" :NewEnumerator0 (Math|Vector|MakeVector 0.0 0.0 (Variables|Jump|GetveticalJumpForce)) :NewEnumerator1 _returnvalue_7 :NewEnumerator2 (* _returnvalue_7 (Variables|Jump|GetRunJumpRatio))) (Variables|Jump|GetSecondaryjumpRatio)) (== (Variables|Jump|GetJumpNumber) (Variables|Default|GetJumpRemaining))) (LocalVariables|GetcurrentJumpT)))

(fn CheckGround
  (bind _returnvalue (Game|GetPlayerCharacter 0))
  (bind _returnvalue_2 (Transformation|GetVelocity _returnvalue))
  (bind _returnvalue_3 (<= (.z _returnvalue_2) 0.0))
  (for _array_element (Components|GetChildrenComponents (Variables|/Game/Player/BP_Character_Game.BP_Character_Game_C|GetArrowContainer (Variables|Default|GetCharacterBP)) false)
    (bind _returnvalue_4 (Collision|LineTraceByChannel (Transformation|GetWorldLocation _array_element) (+ (Transformation|GetWorldLocation _array_element) (* (Math|Vector|GetForwardVector _array_element) 8.0)) "TraceTypeQuery1" false 0 "None"))
    (if _returnvalue_4
      (LocalVariables|SetNumberArrowTrue (+ (LocalVariables|GetNumberArrowTrue) 1))))
  (bind _output_get (Variables|Default|SetisTouchingGround (>= (LocalVariables|GetNumberArrowTrue) 1)))
  (if (Math|Boolean|ANDBoolean _output_get _returnvalue_3 (not (Variables|Default|GetJumping)))
    (Variables|Default|SetJumpRemaining (Variables|Jump|GetJumpNumber))
    (elif (and (Variables|Default|GetJumping) _returnvalue_3)
      (Variables|Default|SetJumping false))))

(fn Jump
  (if (== (Variables|Default|GetJumpRemaining) (Variables|Jump|GetJumpNumber))
    (Variables|Default|SetLastJumpType "NewEnumerator3"))
  (Character|LaunchCharacter (Variables|Default|GetCharacterBP) (.Launch%20Vel (CallFunction|CalculateJumpVelocity (Variables|Default|GetLastJumpType))) true true)
  (Variables|Default|SetLastJumpType (.JumpTypeOut (CallFunction|CalculateJumpVelocity (Variables|Default|GetLastJumpType))))
  (Variables|Default|SetJumpRemaining (- (Variables|Default|GetJumpRemaining) 1))
  (Default|ResetTimer (Variables|Default|GetCoyote))
  (Variables|Default|SetJumping true)
  (Pawn|Components|CharacterMovement|SetMovementMode (Variables|/Script/Engine.Character|GetCharacterMovement (Variables|Default|GetCharacterBP)) "MOVE_Walking" 0))

(fn ReloadSensitivity
  (bind _returnvalue (SaveGame|DoesSaveGameExist "BP_SaveSettings"))
  (if _returnvalue
    (bind _returnvalue_2 (SaveGame|LoadGamefromSlot "BP_SaveSettings"))
    (bind _asbp_save_settings (Utilities|Casting|CastToBP_SaveSettings _returnvalue_2)))
  (Variables|Camera|SetCameraSensitivity (Variables|/Game/Blueprint/BP_SaveSettings.BP_SaveSettings_C|GetSensitivity _asbp_save_settings)))

(fn GetProjectileTransform
  (bind _asbp_character_game (Utilities|Casting|CastToBP_Character_Game (Game|GetPlayerCharacter 0)))
  (bind (_outhit _returnvalue) (Collision|LineTraceByChannel (Transformation|GetWorldLocation (Variables|/Game/Player/BP_Character_Game.BP_Character_Game_C|GetCamera _asbp_character_game)) (+ (Transformation|GetWorldLocation (Variables|/Game/Player/BP_Character_Game.BP_Character_Game_C|GetCamera _asbp_character_game)) (* (Math|Vector|GetForwardVector (Variables|/Game/Player/BP_Character_Game.BP_Character_Game_C|GetCamera _asbp_character_game)) 1e+04)) "TraceTypeQuery1" false 0 "None"))
  (if _returnvalue
    (LocalVariables|SetTargetPos (.ImpactPoint (Collision|BreakHitResult _outhit)))
    (Variables|Default|SetActorHitCameraRC (.HitActor (Collision|BreakHitResult _outhit)))
    (Variables|Default|SetArmAnimRotation (Math|Rotator|FindLookatRotation (Transformation|GetActorLocation _asbp_character_game) (LocalVariables|GetTargetPos)))
    (else
      (LocalVariables|SetTargetPos (+ (Transformation|GetWorldLocation (Variables|/Game/Player/BP_Character_Game.BP_Character_Game_C|GetCamera _asbp_character_game)) (* (Math|Vector|GetForwardVector (Variables|/Game/Player/BP_Character_Game.BP_Character_Game_C|GetCamera _asbp_character_game)) 1e+04)))
      (Variables|Default|SetActorHitCameraRC 0)
      (Variables|Default|SetArmAnimRotation (Math|Rotator|FindLookatRotation (Transformation|GetActorLocation _asbp_character_game) (LocalVariables|GetTargetPos)))))
  (return (Math|Transform|MakeTransform (Transformation|GetActorLocation _asbp_character_game) (Math|Rotator|FindLookatRotation (Transformation|GetActorLocation _asbp_character_game) (LocalVariables|GetTargetPos)))))

(fn Shoot
  (bind _out_transform (CallFunction|GetProjectileTransform))
  (Game|SpawnActorfromClass "/Game/Blueprint/Projectile/BP_Projectile.BP_Projectile_C" _out_transform "Undefined" "MultiplyWithRoot" 0 0)
  (Variables|Default|SetFireflySTime (- (Variables|Default|GetFireflySTime) 1.0))
  (bind _asabp_player (Utilities|Casting|CastToABP_Player (Components|SkeletalMesh|GetAnimInstance (Variables|/Script/Engine.Character|GetMesh (Variables|Default|GetCharacterBP)))))
  (Variables|/Game/Player/ABP_Player.ABP_Player_C|SetisShooting _asabp_player true))

(fn CanShoot
  (return (Math|Boolean|ANDBoolean (Variables|Default|GethasAbilityShoot) (Variables|Default|GetisAiming) (>= (Variables|Default|GetFireflySTime) 1.0))))

(fn GetActorHit
  (bind _characterbp (Variables|Default|GetCharacterBP))
  (bind _camera (Variables|/Game/Player/BP_Character_Game.BP_Character_Game_C|GetCamera _characterbp))
  (bind _returnvalue (Transformation|GetWorldLocation _camera))
  (bind (_outhit _returnvalue_2) (Collision|LineTraceByChannel _returnvalue (+ _returnvalue (* (Math|Vector|GetForwardVector _camera) 3e+03)) "TraceTypeQuery1" false 0 "None"))
  (if _returnvalue_2
    (LocalVariables|SetCurentActorHit (.HitActor (Collision|BreakHitResult _outhit)))
    (else
      (LocalVariables|SetCurentActorHit 0)))
  (return (LocalVariables|GetCurentActorHit)))

(fn CalculateCharacterRotationTarget
  (params (Inputs :type Vector%202D%20Structure) (ForwardV :type Vector) (RightV :type Vector))
  (bind (_x _y) (Math|Vector2D|BreakVector2D Inputs))
  (return (Math|Rotator|FindLookatRotation (Math|Vector|VectorZero) (Math|Vector|Normalize (+ (* ForwardV _y) (* RightV _x))))))

(fn ResetatDeath
  (bind _characterbp (Variables|Default|GetCharacterBP))
  (bind _springarm (Variables|/Game/Player/BP_Character_Game.BP_Character_Game_C|GetSpringArm _characterbp))
  (Default|Aim _characterbp false)
  (Variables|Default|SetisAiming false)
  (Default|UnvisibleCrosshair (Variables|Default|GetCrossHair))
  (Variables|/Script/Engine.SpringArmComponent|SetbEnableCameraRotationLag _springarm (not (Variables|Default|GetisAiming)))
  (Variables|/Script/Engine.SpringArmComponent|SetbEnableCameraLag _springarm (not (Variables|Default|GetisAiming)))
  (CallFunction|StopRunning)
  (Default|Aim (Variables|Default|GetCharacterBP) false)
  (Variables|Default|SetisAiming false)
  (Default|UnvisibleCrosshair (Variables|Default|GetCrossHair))
  (Variables|Character|SetcanRun true)
  (Variables|/Script/Engine.CharacterMovementComponent|SetMaxWalkSpeed (Variables|/Script/Engine.Character|GetCharacterMovement (Variables|Default|GetCharacterBP)) (Variables|Character|GetmaxWalkingSpeed)))

(fn StartRunning
  (if (Variables|Character|GetcanRun)
    (if (not (Variables|Default|GetisRunning))
      (Variables|/Script/Engine.CharacterMovementComponent|SetMaxWalkSpeed (Variables|/Script/Engine.Character|GetCharacterMovement (Variables|Default|GetCharacterBP)) (Variables|Character|GetmaxRunningSpeed))
      (Variables|Default|SetisRunning true))))

(fn StopRunning
  (if (Variables|Default|GetisRunning)
    (Variables|/Script/Engine.CharacterMovementComponent|SetMaxWalkSpeed (Variables|/Script/Engine.Character|GetCharacterMovement (Variables|Default|GetCharacterBP)) (Variables|Character|GetmaxWalkingSpeed))
    (Variables|Default|SetisRunning false)))

(fn EnemyIsinCrosshair
  (bind _actorhit (CallFunction|GetActorHit))
  (return (.bSuccess (Utilities|Casting|CastToBP_FFInteractable _actorhit)) (Math|Float|SelectFloat (.AimMagnetism (Utilities|Struct|BreakSCamType (Variables|/Game/Player/BP_Character_Game.BP_Character_Game_C|GetcurrentCam (Variables|Default|GetCharacterBP)))) 1.0 (.bSuccess (Utilities|Casting|CastToBP_FFInteractable _actorhit)))))