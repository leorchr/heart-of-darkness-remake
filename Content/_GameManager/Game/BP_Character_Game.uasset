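; BP_Character_Game is a playable character with a data-table-driven camera, health, death respawn and tuned jump gravity.
; Tick moves the spring arm after the capsule with optional lag, then snaps the camera to CameraPoint.
; Camera type changes, including aiming, blend arm length, socket offset and FOV along a curve.
; Gravity increases at the jump apex, and lethal damage disables input, then calls controller reset and GameMode respawn.
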(event `self.ReceiveBeginPlay`
  (set `self.Health` (`self.maxHealth`))
  (bind _returnvalue (`|GetDataTableRow` "/Game/DataType/Tables/DT_CamType.DT_CamType" (`KismetStringLibrary.Conv_StringToName` (`|GetEnumeratorNameAsString` (`self.BaseCam`))))
    (:`then`
      (set `self.currentCam` _returnvalue)
      (`self.ChangeCamType` (`self.BaseCam`))
      (set `self.VectorArmOffset` (- (`SceneComponent.K2_GetComponentLocation` (`self.SpringArm`)) (`self.K2_GetActorLocation`))))))

(event `self.ReceiveTick`
  (params (DeltaSeconds :type "Float (single-precision)"))
  (bind _springarm (`self.SpringArm`))
  (bind _returnvalue (+ (`SceneComponent.K2_GetComponentLocation` (`self.CapsuleComponent`)) (`self.VectorArmOffset`)))
  (set `self.Delta Seconds` DeltaSeconds)
  (`SceneComponent.K2_SetWorldTransform` (`self.SpringArm`) (`KismetMathLibrary.MakeTransform` (`KismetMathLibrary.SelectVector` (`KismetMathLibrary.VInterpTo` (`SceneComponent.K2_GetComponentLocation` _springarm) _returnvalue (`self.Delta Seconds`) (`self.CameraLagSpeed`)) _returnvalue (`self.CameraLag`)) (`KismetMathLibrary.SelectRotator` (`KismetMathLibrary.RInterpTo` (`SceneComponent.K2_GetComponentRotation` _springarm) (`self.TargetArmRotation`) (`self.Delta Seconds`) (`self.CameraLagRotSpeed`)) (`self.TargetArmRotation`) (`self.CameraLag`))) false false)
  (`SceneComponent.K2_SetWorldTransform` (`self.Camera`) (`SceneComponent.K2_GetComponentToWorld` (`self.CameraPoint`)) false false)
  (if (!= (`self.camTT`) 0.0)
    (`self.CamTransitionTick` (`self.Delta Seconds`))))

(event `self.K2_OnMovementModeChanged`
  (params (PrevMovementMode :type "EMovementMode Enum" :default "MOVE_None") (NewMovementMode :type "EMovementMode Enum" :default "MOVE_None") (PrevCustomMode :type Byte) (NewCustomMode :type Byte))
  (bind _charactermovement (`self.CharacterMovement`))
  ;[0.05098 0.05098 0.05098] Apex
  (bind _output_get (set `CharacterMovementComponent.bNotifyApex` (`|EnumEquality` NewMovementMode "MOVE_Falling") _charactermovement))
  (if _output_get
    (set `CharacterMovementComponent.GravityScale` 1.0 _charactermovement)
    (add `self.OnReachedJumpApex` (delegate `ApexReached`))
    (else
      (clear `self.OnReachedJumpApex`))))

(event `Death`
  (bind _returnvalue (`GameplayStatics.GetPlayerController` 0))
  ;[0.3281 0.06836 0.06836] Death Case
  (`self.DisableInput` _returnvalue _returnvalue)
  (bind _asbp_controller_game (cast `/Game/_GameManager/Game/BP_Controller_Game` _returnvalue))
  (`/Game/_GameManager/Game/BP_Controller_Game.ResetAtDeath` _asbp_controller_game)
  (bind _asbp_gm_game (cast `/Game/_GameManager/Game/BP_GM_Game` (`GameplayStatics.GetGameMode`)))
  (`/Game/_GameManager/Game/BP_GM_Game.Respawn Player` :`self` _asbp_gm_game))

(event `ApexReached`
  ;[0.05098 0.05098 0.05098] Apex
  (`KismetSystemLibrary.PrintString` "Apex")
  (set `CharacterMovementComponent.GravityScale` 1.75 (`self.CharacterMovement`)))

(event `self.ReceiveAnyDamage`
  (params (Damage :type "Float (single-precision)") (DamageType :type "DamageType Object Reference") (InstigatedBy :type "Controller Object Reference") (DamageCauser :type "Actor Object Reference"))
  ;[0.06798 0.5677 0.1489] On Any Damage remove health and check if dead
  (set `self.Health` (- (`self.Health`) Damage))
  (if (<= (`self.Health`) 0.0)
    (`self.Death`)))

(fn `Aim`
  (params (`Aim?` :type Boolean))
  (if `Aim?`
    (`self.ChangeCamType` "NewEnumerator2")
    (else
      (`self.ChangeCamType` (`self.BaseCam`)))))

(fn `ChangeBaseCam`
  (params (`New Cam Type` :type "/Game/DataType/ECamType Enum" :default "NewEnumerator0"))
  (set `self.BaseCam` `New Cam Type`))

(fn `ChangeCamType`
  (params (Enum :type "/Game/DataType/ECamType Enum" :default "NewEnumerator0"))
  (bind _springarm (`self.SpringArm`))
  (bind (_currentcam_enum _currentcam_targetarmlength _currentcam_socketoffset _currentcam_camerafov _currentcam_cameralag _currentcam_cameralagspeed _currentcam_cameralagrspeed _currentcam_sensitivitymultiplier) (break `/Game/DataType/SCamType` (`self.currentCam`)))
  (set `self.lastCam` (make `/Game/DataType/SCamType` _currentcam_enum (`SpringArmComponent.TargetArmLength` _springarm) (`SpringArmComponent.SocketOffset` _springarm) (`CameraComponent.FieldOfView` (`self.Camera`)) _currentcam_cameralag _currentcam_cameralagspeed _currentcam_cameralagrspeed _currentcam_sensitivitymultiplier))
  (bind _returnvalue (`|GetDataTableRow` (`self.camDT`) (`KismetStringLibrary.Conv_StringToName` (`|GetEnumeratorNameAsString` Enum)))
    (:`then`
      (bind _output_get (set `self.currentCam` _returnvalue))
      (set `self.camTT` (`self.camTransitionTime`))
      (bind (_enum _targetarmlength _socketoffset _camerafov _cameralag _cameralagspeed _cameralagrspeed) (break `/Game/DataType/SCamType` _output_get))
      (set `self.CameraLag` _cameralag)
      (set `self.CameraLagSpeed` _cameralagspeed)
      (set `self.CameraLagRotSpeed` _cameralagrspeed)
      (return))))

(fn `UserConstructionScript`)